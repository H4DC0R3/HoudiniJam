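; BP_MIDI_Test is a placeholder test Blueprint that visualises three shot events as coloured debug lines, apparently for MIDI-driven triggering.
; The custom events Shot1, Shot2 and Shot3 each pass a distinct colour to the TraceLine function.
; TraceLine draws a brief, thick debug line forward from the Arrow component, with no collision query despite its name.
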(event `Shot 1`
  (`self.TraceLine` (struct :`R` 0.84375 :`G` 0.004395 :`B` 0.004395 :`A` 1.0)))

(event `Shot 2`
  (`self.TraceLine` (struct :`R` 0.330572 :`B` 1.0 :`A` 1.0)))

(event `Shot 3`
  (`self.TraceLine` (struct :`G` 0.979828 :`B` 1.0 :`A` 1.0)))

(fn `TraceLine`
  (params (TraceColor :type "LinearColor Structure"))
  (bind _arrow (`self.Arrow`))
  (bind _returnvalue (`SceneComponent.K2_GetComponentLocation` _arrow))
  (`KismetSystemLibrary.DrawDebugLine` _returnvalue (+ _returnvalue (* (`KismetMathLibrary.GetForwardVector` (`SceneComponent.K2_GetComponentRotation` _arrow)) 1000.0)) TraceColor 0.1 10.0))

(fn `UserConstructionScript`)