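; Music-reactive spawner that surrounds itself with stacked rings of randomly spaced, inward-facing cannons and fires them to a looping track.
; The construction script previews the layout with instanced meshes, which BeginPlay clears before spawning BP_MIDI_Test actors at newly randomized angles, each on a random channel.
; During playback, precomputed loudness at the current time selects one of three bands, triggering that channel's cannons with its own shot type.
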(event `self.ReceiveBeginPlay`
  (bind (_returnvalue_x _returnvalue_y) (`KismetMathLibrary.BreakVector` (`self.K2_GetActorLocation`)))
  (bind _audio (`self.Audio`))
  (bind _cannon (`self.Cannon`))
  (bind _quantity (`self.Quantity`))
  (`|ExecutionSequence`
    (:`then_0`
      (`InstancedStaticMeshComponent.ClearInstances` (`self.InstancedStaticMesh`))
      (for _array_element _cannon
        (`self.K2_DestroyActor` _array_element))
      (`KismetArrayLibrary.Array_Clear` _cannon)
      (for _index (range (`self.SizeTop`))
        (for _index_2 (range (+ _quantity 1))
          (bind _returnvalue (* _index (`self.TopHeightPerStep`)))
          (bind _returnvalue_2 (+ (* (`KismetMathLibrary.GetForwardVector` (`KismetMathLibrary.MakeRotator` 0.0 0.0 (+ (`KismetMathLibrary.Conv_IntToDouble` (* _index_2 (/ 360 _quantity))) (`KismetMathLibrary.Conv_IntToDouble` (* (- _index_2 1) (`KismetMathLibrary.RandomIntegerInRange` 10 40)))))) (`self.Radius`)) (`self.K2_GetActorLocation`) (`KismetMathLibrary.MakeVector` 0.0 0.0 _returnvalue)))
          (`self.SpawnCannon` (`KismetMathLibrary.MakeTransform` _returnvalue_2 (`KismetMathLibrary.FindLookAtRotation` _returnvalue_2 (`KismetMathLibrary.MakeVector` _returnvalue_x _returnvalue_y _returnvalue)))))))
    (:`then_1`
      (add `AudioComponent.OnAudioPlaybackPercent` _audio (delegate `Event`))
      (add `AudioComponent.OnAudioFinished` _audio (delegate `OnAudioFinished_Event_0`))
      (`AudioComponent.Play` _audio 0.0 :!label _label))))

(event `OnAudioFinished_Event_0`
  (goto _label))

(event `Event`
  (params (PlayingSoundWave :type "SoundWave Object Reference") (PlaybackPercent :type "Float (double-precision)"))
  (bind _outloudness (`LoudnessNRT.GetNormalizedChannelLoudnessAtTime` (`self.Loudnessfile`) (* PlaybackPercent (`self.Duration`)) 0))
  (if (<= _outloudness 0.1)
    _
    (elif (and (>= _outloudness 0.11) (<= _outloudness 0.6))
      (for _array_element (`self.Cannon`)
        (if (== (`/Game/Assets/PlaceHolder/Blueprint/BP_MIDI_Test.Channel` _array_element) 0)
          (`/Game/Assets/PlaceHolder/Blueprint/BP_MIDI_Test.Shot 1` _array_element)))
      (elif (and (>= _outloudness 0.61) (<= _outloudness 0.94))
        (for _array_element_2 (`self.Cannon`)
          (if (== (`/Game/Assets/PlaceHolder/Blueprint/BP_MIDI_Test.Channel` _array_element_2) 1)
            (`/Game/Assets/PlaceHolder/Blueprint/BP_MIDI_Test.Shot 2` _array_element_2)))
        (elif (and (>= _outloudness 0.95) (<= _outloudness 1.0))
          (for _array_element_3 (`self.Cannon`)
            (if (== (`/Game/Assets/PlaceHolder/Blueprint/BP_MIDI_Test.Channel` _array_element_3) 2)
              (`/Game/Assets/PlaceHolder/Blueprint/BP_MIDI_Test.Shot 3` _array_element_3))))))))

(fn `SpawnCannon`
  (params (SpawnTransform :type "Transform Structure"))
  (bind _returnvalue (`|SpawnActorFromClass` "/Game/Assets/PlaceHolder/Blueprint/BP_MIDI_Test.BP_MIDI_Test_C" SpawnTransform "AlwaysSpawn" "OverrideRootScale" null (`self.Loudnessfile`) (`KismetMathLibrary.RandomIntegerInRange` 0 2) null))
  (`KismetArrayLibrary.Array_Add` (`self.Cannon`) _returnvalue))

(fn `UserConstructionScript`
  (bind (_returnvalue_x _returnvalue_y) (`KismetMathLibrary.BreakVector` (`self.K2_GetActorLocation`)))
  (bind _quantity (`self.Quantity`))
  (bind _sound (`AudioAnalyzerNRT.Sound` (`self.Loudnessfile`)))
  (`AudioComponent.SetSound` (`self.Audio`) _sound)
  (set `self.Duration` (`SoundBase.Duration` _sound))
  (`InstancedStaticMeshComponent.ClearInstances` (`self.InstancedStaticMesh`))
  (for _index (range (`self.SizeTop`))
    (for _index_2 (range (+ _quantity 1))
      (bind _returnvalue (* _index (`self.TopHeightPerStep`)))
      (bind _returnvalue_2 (+ (* (`KismetMathLibrary.GetForwardVector` (`KismetMathLibrary.MakeRotator` 0.0 0.0 (+ (`KismetMathLibrary.Conv_IntToDouble` (* _index_2 (/ 360 _quantity))) (`KismetMathLibrary.Conv_IntToDouble` (* (+ _index_2 1) (`KismetMathLibrary.RandomIntegerInRange` 0 40)))))) (`self.Radius`)) (`self.K2_GetActorLocation`) (`KismetMathLibrary.MakeVector` 0.0 0.0 _returnvalue)))
      (`InstancedStaticMeshComponent.AddInstance` (`self.InstancedStaticMesh`) (`KismetMathLibrary.MakeTransform` _returnvalue_2 (`KismetMathLibrary.FindLookAtRotation` _returnvalue_2 (`KismetMathLibrary.MakeVector` _returnvalue_x _returnvalue_y _returnvalue)))))))