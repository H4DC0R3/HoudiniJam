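; BP_PlatarformPlace procedurally lays out instanced meshes, apparently platforms, in a rising ring or spiral.
; The construction script adds Quantity instances at a set Radius, stepping height per index and spreading yaw evenly plus seeded random spacing scaled by index.
; Each instance's rotation combines a look-at toward the actor's XY location with a yaw of index times Seed.
; The event graph is empty.
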(fn `UserConstructionScript`
  (bind (_returnvalue_x _returnvalue_y) (`KismetMathLibrary.BreakVector` (`self.K2_GetActorLocation`)))
  (bind _returnvalue (- (`self.Quantity`) 1))
  (`KismetMathLibrary.SetRandomStreamSeed` (`self.SeedStream`) (`self.Seed`))
  (for _index (range (+ _returnvalue 1))
    (bind _returnvalue_2 (- _index 1))
    (bind _returnvalue_3 (* _returnvalue_2 (`self.TopHeightPerStep`)))
    (bind _returnvalue_4 (+ (* (`KismetMathLibrary.GetForwardVector` (`KismetMathLibrary.MakeRotator` 0.0 0.0 (+ (`KismetMathLibrary.Conv_IntToDouble` (* _index (/ 360 _returnvalue))) (* _returnvalue_2 (`KismetMathLibrary.RandomFloatInRangeFromStream` (`self.Distance Min`) (`self.Distancec Max`) (`self.SeedStream`)))))) (`self.Radius`)) (`KismetMathLibrary.MakeVector` 0.0 0.0 _returnvalue_3)))
    (`InstancedStaticMeshComponent.AddInstance` (`self.InstancedStaticMesh`) (`KismetMathLibrary.MakeTransform` _returnvalue_4 (`KismetMathLibrary.ComposeRotators` (`KismetMathLibrary.FindLookAtRotation` _returnvalue_4 (`KismetMathLibrary.MakeVector` _returnvalue_x _returnvalue_y _returnvalue_3)) (`KismetMathLibrary.MakeRotator` 0.0 0.0 (* _index (`KismetMathLibrary.Conv_IntToDouble` (`self.Seed`)))))))))