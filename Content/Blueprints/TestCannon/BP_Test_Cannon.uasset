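; Test cannon that fires bullets in time with a looping sound, driven by its loudness.
; Construction copies the LoudnessAnalyzer's sound and duration to the Audio component, whose playback callback samples normalized loudness at the current time.
; The Channel variable picks which loudness band triggers this cannon: low, mid or high, each spawning its own bullet class at the Arrow.
; Each shot type has a DoOnce-and-Delay cooldown; SpawnBullet ignores its TraceColor input.
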(event `self.ReceiveBeginPlay`
  (bind _audio (`self.Audio`))
  (add `AudioComponent.OnAudioPlaybackPercent` _audio (delegate `Event`))
  (add `AudioComponent.OnAudioFinished` _audio (delegate `OnAudioFinished_Event_0`))
  ;[1 1 1] Loop Sound
  (`AudioComponent.Play` _audio 0.0 :!label _label))

(event `OnAudioFinished_Event_0`
  (goto _label))

(event `Event`
  (params (PlayingSoundWave :type "SoundWave Object Reference") (PlaybackPercent :type "Float (double-precision)"))
  (bind _outloudness (`LoudnessNRT.GetNormalizedChannelLoudnessAtTime` (`self.LoudnessAnalyzer`) (* PlaybackPercent (`self.Duration`)) 0))
  (if (<= _outloudness 0.1)
    _
    (elif (and (>= _outloudness 0.11) (<= _outloudness 0.6) (== (`self.Channel`) 0))
      (`/Engine/EditorBlueprintResources/StandardMacros.DoOnce` false :!label _label_2
        (:`Completed`
          (`self.Shot Low`)
          (`KismetSystemLibrary.Delay` 0.5)
          (goto _label_2 :!via `Reset`)))
      (elif (and (>= _outloudness 0.61) (<= _outloudness 0.94) (== (`self.Channel`) 1))
        (`/Engine/EditorBlueprintResources/StandardMacros.DoOnce` false :!label _label_3
          (:`Completed`
            (`self.Shot Mid`)
            (`KismetSystemLibrary.Delay` 0.5)
            (goto _label_3 :!via `Reset`)))
        (elif (and (>= _outloudness 0.95) (<= _outloudness 1.0) (== (`self.Channel`) 2))
          (`/Engine/EditorBlueprintResources/StandardMacros.DoOnce` false :!label _label_4
            (:`Completed`
              (`self.Shot High`)
              (`KismetSystemLibrary.Delay` 0.5)
              (goto _label_4 :!via `Reset`))))))))

(event `Shot Low`
  (`self.SpawnBullet` (struct :`R` 0.84375 :`G` 0.004395 :`B` 0.004395 :`A` 1.0) (`self.BulletLowFrequency`)))

(event `Shot Mid`
  (`self.SpawnBullet` (struct :`R` 0.330572 :`B` 1.0 :`A` 1.0) (`self.BulletMidFrequency`)))

(event `Shot High`
  (`self.SpawnBullet` (struct :`G` 0.979828 :`B` 1.0 :`A` 1.0) (`self.BulletHighFrequency`)))

(fn `SpawnBullet`
  (params (TraceColor :type "LinearColor Structure") (Class :type "Actor Class Reference"))
  (`|SpawnActorFromClass` Class (`KismetMathLibrary.MakeTransform` (`SceneComponent.K2_GetComponentLocation` (`self.Arrow`)) (`SceneComponent.K2_GetComponentRotation` (`self.Arrow`))) "Undefined" "OverrideRootScale" null null))

(fn `UserConstructionScript`
  (bind _sound (`AudioAnalyzerNRT.Sound` (`self.LoudnessAnalyzer`)))
  (`AudioComponent.SetSound` (`self.Audio`) _sound)
  (set `self.Duration` (`SoundBase.Duration` _sound)))