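; Test cannon manager that fires groups of cannons on a musical tempo, split into low, mid and high bands.
; The construction script derives each band's delay from its BPM and a note-division multiplier, though the high band reads the mid band's division.
; BeginPlay starts three looping timers, each calling SpawnBullet on every cannon in its band's array with that band's bullets.
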(event `Spawn Bullet Mid`
  (for _array_element (`self.CannonBPM_Mid`)
    (`/Game/Blueprints/BP_CannonByFloat.SpawnBullet` _array_element (`self.Bullets_Mid`))))

(event `self.ReceiveBeginPlay`
  (`KismetSystemLibrary.K2_SetTimerDelegate` (delegate `Spawn Bullet Low`) (`self.Delay_Low`) true)
  (`KismetSystemLibrary.K2_SetTimerDelegate` (delegate `Spawn Bullet Mid`) (`self.Delay_Mid`) true)
  (`KismetSystemLibrary.K2_SetTimerDelegate` (delegate `Spawn Bullet High`) (`self.Delay_High`) true))

(event `Spawn Bullet Low`
  (for _array_element (`self.CannonBPM_Low`)
    (`/Game/Blueprints/BP_CannonByFloat.SpawnBullet` _array_element (`self.Bullets_Low`))))

(event `Spawn Bullet High`
  (for _array_element (`self.CannonBPM_High`)
    (`/Game/Blueprints/BP_CannonByFloat.SpawnBullet` _array_element (`self.Bullets_High`))))

(fn `UserConstructionScript`
  (set `self.Delay_Low` (/ 60.0 (* (`self.BPM_Low`) (select `/Game/Blueprints/Resource/BeatTime` (`self.Time_Low`) :`NewEnumerator0` 2.0 :`NewEnumerator1` 4.0 :`NewEnumerator2` 8.0 :`NewEnumerator3` 16.0 :!type "Float (single-precision)"))))
  (set `self.Delay_Mid` (/ 60.0 (* (`self.BPM_Mid`) (select `/Game/Blueprints/Resource/BeatTime` (`self.Time_Mid`) :`NewEnumerator0` 2.0 :`NewEnumerator1` 4.0 :`NewEnumerator2` 8.0 :`NewEnumerator3` 16.0 :!type "Float (single-precision)"))))
  (set `self.Delay_High` (/ 60.0 (* (`self.BPM_High`) (select `/Game/Blueprints/Resource/BeatTime` (`self.Time_Mid`) :`NewEnumerator0` 2.0 :`NewEnumerator1` 4.0 :`NewEnumerator2` 8.0 :`NewEnumerator3` 16.0 :!type "Float (single-precision)")))))