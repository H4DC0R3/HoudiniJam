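; BP_SawBlade is a short-lived saw blade hazard that kills a DynamicCharacter overlapping its collision component.
; After a brief delay to avoid colliding with its cannon, a fast looping timer box-traces around the mesh for static and dynamic world objects, ignoring the player.
; A hit spawns an explosion particle and destroys the blade.
; Otherwise, it destroys itself after a fixed lifetime.
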(event `self.ReceiveBeginPlay`
  (`|ExecutionSequence`
    (:`then_0`
      (`KismetSystemLibrary.Delay` 10.0)
      (`self.K2_DestroyActor`))
    (:`then_1`
      (`KismetSystemLibrary.Delay` 0.5) ; Add thisd Delay to fix collide with cannon
      (`KismetSystemLibrary.K2_SetTimerDelegate` (delegate `Destroy on Terrain`) 0.05 true))))

(event `Destroy on Terrain`
  (bind _returnvalue (`SceneComponent.K2_GetComponentLocation` (`self.StaticMesh`)))
  (bind (_outhit _returnvalue_2) (`KismetSystemLibrary.BoxTraceSingleForObjects` _returnvalue (+ _returnvalue (0.0 0.0 1.0)) (100.0 100.0 10.0) (struct) (`|MakeArray` "ObjectTypeQuery1" "ObjectTypeQuery2" :!type "EObjectTypeQuery Enum") false (`|MakeArray` (`GameplayStatics.GetPlayerCharacter` 0) :!type "Actor Object Reference") "None" true (struct :`R` 1.0 :`A` 1.0) (struct :`G` 1.0 :`A` 1.0) 1.0))
  (if _returnvalue_2
    (`GameplayStatics.SpawnEmitterAtLocation` "/Game/Particles/PS_ExplodeSaw.PS_ExplodeSaw" (`.Location` (`GameplayStatics.BreakHitResult` _outhit)))
    (`self.K2_DestroyActor`)))

(event `self.SM_SawBlade_Collision.OnComponentBeginOverlap`
  (params (OverlappedComponent :type "PrimitiveComponent Object Reference") (OtherActor :type "Actor Object Reference") (OtherComp :type "PrimitiveComponent Object Reference") (OtherBodyIndex :type Integer) (bFromSweep :type Boolean) (SweepResult :type "HitResult Structure (by ref)"))
  ;[1 1 1] Kill Player
  (bind _asdynamic_character (cast `/Game/DynamicLocomotion/Blueprints/DynamicCharacter` OtherActor))
  (`/Game/DynamicLocomotion/Blueprints/DynamicCharacter.Die` _asdynamic_character))

(fn `UserConstructionScript`)