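; BP_Cannon is a cannon that fires one of three bullet classes: low, mid or high frequency.
; The ShotLow, ShotMid and ShotHigh events each pass their bullet class and a color to SpawnBullet.
; SpawnBullet spawns that class at the Arrow component's world location and rotation with unit scale.
; The TraceColor input and a forward endpoint calculation from the Arrow are left unused.
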(event `Shot Low`
  (`self.SpawnBullet` (struct :`R` 0.84375 :`G` 0.004395 :`B` 0.004395 :`A` 1.0) (`self.BulletLowFrequency`)))

(event `Shot Mid`
  (`self.SpawnBullet` (struct :`R` 0.330572 :`B` 1.0 :`A` 1.0) (`self.BulletMidFrequency`)))

(event `Shot High`
  (`self.SpawnBullet` (struct :`G` 0.979828 :`B` 1.0 :`A` 1.0) (`self.BulletHighFrequency`)))

(fn `SpawnBullet`
  (params (TraceColor :type "LinearColor Structure") (Class :type "Actor Class Reference"))
  (`|SpawnActorFromClass` Class (`KismetMathLibrary.MakeTransform` (`SceneComponent.K2_GetComponentLocation` (`self.Arrow`)) (`SceneComponent.K2_GetComponentRotation` (`self.Arrow`))) "Undefined" "OverrideRootScale" null null))

(fn `UserConstructionScript`)