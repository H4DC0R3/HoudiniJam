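; BP_Checkpoint is a checkpoint actor that records a respawn point when a DynamicCharacter enters its trigger box.
; On overlap it stores the Cube's world transform as the character's LastCheckpoint and spawns a particle effect at the TextRender's location.
; A shared flag then blocks retriggering by any actor until a delay ends.
; The construction script fixes the Cube to an absolute, vertically stretched scale.
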(event `self.Box.OnComponentBeginOverlap`
  (params (OverlappedComponent :type "PrimitiveComponent Object Reference") (OtherActor :type "Actor Object Reference") (OtherComp :type "PrimitiveComponent Object Reference") (OtherBodyIndex :type Integer) (bFromSweep :type Boolean) (SweepResult :type "HitResult Structure (by ref)"))
  (if (not (`self.Block Checkpoint`))
    (bind _asdynamic_character (cast `/Game/DynamicLocomotion/Blueprints/DynamicCharacter` OtherActor))
    (set `/Game/DynamicLocomotion/Blueprints/DynamicCharacter.LastCheckpoint` (`SceneComponent.K2_GetComponentToWorld` (`self.Cube`)) _asdynamic_character)
    (set `self.Block Checkpoint` true)
    (`GameplayStatics.SpawnEmitterAtLocation` "/Game/Particles/PS_Checkpoint.PS_Checkpoint" (`SceneComponent.K2_GetComponentLocation` (`self.TextRender`)))
    (`KismetSystemLibrary.Delay` 30.0)
    (set `self.Block Checkpoint` false)))

(fn `UserConstructionScript`
  (bind _cube (`self.Cube`))
  (set `SceneComponent.bAbsoluteScale` true _cube)
  (`SceneComponent.SetRelativeScale3D` _cube (1.0 1.0 1.8))
  (`SceneComponent.SetWorldScale3D` _cube (1.0 1.0 1.8)))