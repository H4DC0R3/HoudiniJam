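; BP_CannonByFloat is a cannon that repeatedly spawns a bullet actor at a tempo-based interval.
; Its construction script sets the timer delay by dividing BPM by 2, 4, 8 or 16, chosen by the Time selection.
; On BeginPlay a looping timer calls SpawnBullet, which spawns BulletBP at the Arrow component's world location and rotation.
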(event `self.ReceiveBeginPlay`
  (`KismetSystemLibrary.K2_SetTimerDelegate` (delegate `Spawn Bullet`) (`self.DelayTime`) true))

(event `Spawn Bullet`
  (`self.SpawnBullet` (`self.BulletBP`)))

(fn `SpawnBullet`
  (params (Class :type "Actor Class Reference"))
  (`|SpawnActorFromClass` Class (`KismetMathLibrary.MakeTransform` (`SceneComponent.K2_GetComponentLocation` (`self.Arrow`)) (`SceneComponent.K2_GetComponentRotation` (`self.Arrow`))) "Undefined" "OverrideRootScale" null null))

(fn `UserConstructionScript`
  (set `self.DelayTime` (/ (`self.BPM`) (select `/Game/Blueprints/Resource/BeatTime` (`self.Time`) :`NewEnumerator0` 2.0 :`NewEnumerator1` 4.0 :`NewEnumerator2` 8.0 :`NewEnumerator3` 16.0 :!type "Float (single-precision)"))))